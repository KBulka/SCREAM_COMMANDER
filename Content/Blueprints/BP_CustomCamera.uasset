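; BP_CustomCamera is a camera Blueprint that drives an on-screen compass from the direction the camera faces.
; Each Tick adds the calibration offset KalibracjaKompasa to the camera component's world yaw and converts the sum from degrees to a fraction of a turn.
; The result sets the "Compass Rotation" scalar on the dynamic material of the Compass widget's CompassImage.
; BeginPlay and the construction script only call their parent versions.
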(event EventBeginPlay
  (|CallParentFunction))

(event Collision|EventActorBeginOverlap
  (params (OtherActor :type Actor%20Object%20Reference))
  (|CallParentFunction OtherActor) ; Ten węzeł jest wyłączony i nie będzie wywoływany.\nPrzeciągnij gniazda, aby utworzyć funkcjonalność.
)

(event EventTick
  (params (DeltaSeconds :type Float%20%28single-precision%29))
  (|CallParentFunction DeltaSeconds)
  (bind _returnvalue (Appearance|GetDynamicMaterial (Variables|/Game/Blueprints/UI/BP_Compas.BP_Compas_C|GetCompass_Image (Variables|Default|GetCompass)) :!class /Script/UMG.Image))
  (Rendering|Material|SetScalarParameterValue _returnvalue "Compass Rotation" (/ (+ (.yaw (Transformation|GetWorldRotation (Variables|Default|GetCameraComponent))) (Variables|Default|GetKalibracjaKompasa)) 3.6e+02) :!class /Script/Engine.MaterialInstanceDynamic))

(fn ConstructionScript
  (|CallParentFunction))