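; Voice-commanded character Blueprint (enamy, speaking as "Mike") that moves by spoken direction and can take damage.
; NewVoiceTaskEvent matches keywords in VoiceTask to set MoveType and prints a reply; Tick applies continuous movement input along the actor's axes until changed or stopped.
; Health functions forward to BPCDamageSystem, except GetCurrentHealth, which returns zero.
; Component death and damage-response events are bound in the construction script and only print debug text.
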(event Custom|Death
  (Development|PrintString "DEAD"))

(event Custom|NewVoiceTaskEvent
  (CallFunction|MovmentFunction))

(event Custom|Damage%20Response
  (params (DamageResponse :type E_DamageResponses%20Enum :default "NewEnumerator0"))
  (Development|PrintString (Utilities|String|EnumtoString DamageResponse)))

(event EventTick
  (params (DeltaSeconds :type Float%20%28single-precision%29))
  (switch int (Variables|Default|GetMove_type)
    (:1
      (Pawn|Input|AddMovementInput (Transformation|GetActorForwardVector) 1.0 false))
    (:2
      (Pawn|Input|AddMovementInput (Math|Vector|NegateVector (Transformation|GetActorForwardVector)) 1.0 false))
    (:3
      (Pawn|Input|AddMovementInput (Transformation|GetActorRightVector) 1.0 false))
    (:4
      (Pawn|Input|AddMovementInput (Math|Vector|NegateVector (Transformation|GetActorRightVector)) 1.0 false))))

(fn ConstructionScript
  (bind _bpc_damagesystem (Variables|Default|GetBPC_DamageSystem))
  (EventDispatchers|BindEventtoOnDeath _bpc_damagesystem (EventDispatchers|CreateEvent :!event Custom|Death))
  (EventDispatchers|BindEventtoDamageResponse _bpc_damagesystem (EventDispatchers|CreateEvent :!event Custom|Damage%20Response)))

(fn MovmentFunction
  (bind _voice_task (Variables|Default|Getvoice_task))
  (if (Utilities|String|Contains _voice_task "right")
    (Development|PrintString "Mike: im going right")
    (Variables|Default|SetMove_type 3)
    (elif (Utilities|String|Contains _voice_task "left")
      (Development|PrintString "Mike: im going left")
      (Variables|Default|SetMove_type 4)
      (elif (Utilities|String|Contains _voice_task "forward")
        (Development|PrintString "Mike: im going forward")
        (Variables|Default|SetMove_type 1)
        (elif (Utilities|String|Contains _voice_task "backward")
          (Development|PrintString "Mike: im going backward")
          (Variables|Default|SetMove_type 2)
          (elif (Utilities|String|Contains _voice_task "stop")
            (Development|PrintString "Mike: im stopping")
            (Variables|Default|SetMove_type 0)))))))

(fn GetCurrentHealth
  (params (Amount :type Integer))
  (return 0))

(fn GetMaxHealth
  (return (Variables|/Game/DamageSystem/BPC_DamageSystem.BPC_DamageSystem_C|GetMaxHealth (Variables|Default|GetBPC_DamageSystem))))

(fn Heal
  (params (Amount :type Integer))
  (bind _heal (Default|Heal (Variables|Default|GetBPC_DamageSystem) Amount))
  (return _heal))

(fn TakeDamage
  (params (DamageInfo :type S%20Damage%20Info%20Structure))
  (bind _wasdamaged (Default|TakeDamage (Variables|Default|GetBPC_DamageSystem) DamageInfo))
  (return _wasdamaged))