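; BasicAttacks is a component that gives its owning actor projectile, laser and beam attacks.
; AttackSimple runs a looping timer that fires projectiles with random yaw and speed until the attack limit, then calls SimpleAttackEnd after a short delay.
; LaserAttack spawns a laser and damages the target immediately, while Skill_Beam_Event spawns a beam with or without a valid target.
; MachineGunAttack is an empty stub.
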(event Custom|LaserAttack
  (params (AttackTarget :type Actor%20Object%20Reference) (DamageAmount :type Float%20%28double-precision%29))
  (bind _returnvalue (Components|GetOwner))
  (Variables|Default|SetAttackTarget AttackTarget)
  (Variables|Default|SetDamage%20Amount DamageAmount)
  (Game|SpawnActorfromClass "/Game/DamageSystem/Laser/BP_Laser_Base.BP_Laser_Base_C" (Transformation|GetActorTransform _returnvalue) "Undefined" "MultiplyWithRoot" 0 (Variables|Default|GetAttackTarget) _returnvalue 0)
  (Class|BPDamageable|TakeDamage(Message) (Variables|Default|GetAttackTarget) (Utilities|Struct|MakeS_DamageInfo (Math|Float|Truncate (Variables|Default|GetDamage%20Amount)) "NewEnumerator0" "NewEnumerator0" false false)))

(event Custom|MachineGunAttack)

(event Custom|Skill_Beam_Event
  (params (AttackTarget :type Actor%20Object%20Reference) (Damage :type Float%20%28double-precision%29))
  (bind _returnvalue (Components|GetOwner))
  (bind _returnvalue_2 (Transformation|GetActorTransform _returnvalue))
  (bind _output_get (Variables|Default|SetAttackTarget AttackTarget))
  (if (Utilities|IsValid _output_get)
    (Game|SpawnActorfromClass "/Game/DamageSystem/Skills/Skill_Beam.Skill_Beam_C" (Math|Transform|MakeTransform (Math|Vector|MakeVector (.x (.location _returnvalue_2)) (.y (.location _returnvalue_2)) (.z (.location _returnvalue_2))) (.rotation _returnvalue_2) (.scale _returnvalue_2)) "Undefined" "MultiplyWithRoot" 0 (Variables|Default|GetAttackTarget) _returnvalue 0)
    (Utilities|FlowControl|Delay 2.0)
    (else
      (Game|SpawnActorfromClass "/Game/DamageSystem/Skills/Skill_Beam.Skill_Beam_C" (Transformation|GetActorTransform _returnvalue) "Undefined" "MultiplyWithRoot" 0 0 _returnvalue 0))))

(event Custom|AttackSimple
  (params (target :type Actor%20Object%20Reference) (AttackLimt :type Integer) (TimeInterval :type Float%20%28double-precision%29) (Gravity :type Float%20%28double-precision%29) (Speed :type Float%20%28double-precision%29) (Damage%20Amount :type Float%20%28double-precision%29))
  (Variables|Default|SetAttackTarget target)
  (Variables|Default|SetAttackLimit AttackLimt)
  (Variables|Default|SetTimeInterval TimeInterval)
  (Variables|Default|SetGravity Gravity)
  (Variables|Default|SetSpeed Speed)
  (Variables|Default|SetDamage%20Amount Damage%20Amount)
  ;[1 1 1] Powtarzaj Atak  o {Time}
  (bind _returnvalue (Utilities|Time|SetTimerbyEvent (delegate Custom|AttackSimpleLoop) (Variables|Default|GetTimeInterval) true)))

(event Custom|AttackSimpleLoop
  (bind _returnvalue (Components|GetOwner))
  (bind _returnvalue_2 (Transformation|GetActorTransform _returnvalue))
  (bind (_location _rotation _scale) (Math|Transform|BreakTransform _returnvalue_2))
  (bind (_roll _pitch _yaw) (Math|Rotator|BreakRotator _rotation))
  ;[1 1 1] Powtarzaj Atak  o {Time}
  (bind _returnvalue_3 (Game|SpawnActorfromClass "/Game/Projectiles/BP_Projectal_Child.BP_Projectal_Child_C" (Math|Transform|MakeTransform _location (Math|Rotator|MakeRotator _roll _pitch (+ _yaw (Math|Random|RandomFloatinRange -1e+01 1e+01))) _scale) "Undefined" "MultiplyWithRoot" (Components|GetOwner) (Variables|Default|GetDamage%20Amount) (Variables|Default|GetGravity) (+ (Variables|Default|GetSpeed) (Math|Random|RandomFloatinRange -4e+02 1e+03)) (Variables|Default|GetAttackTarget) false 0))
  ;[1 1 1] Sprawdza czy została wykonane {Attack Limit} ataków. Jeżeli tak przerywa event loop
  (bind _result (Math|Integer|IncrementInt (Variables|Default|GetAttackCount))
    (:%20%20
      (bind _output_get (Variables|Default|SetAttackCount _result))
      (if (== _output_get (Variables|Default|GetAttackLimit))
        (Variables|Default|SetAttackCount 0)
        (Utilities|Time|ClearandInvalidateTimerbyHandle (stale Custom|AttackSimple _returnvalue))
        (Utilities|FlowControl|Delay 0.1)
        (Default|CallSimpleAttackEnd)))))