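; Charlie_NPC is an NPC Blueprint that moves continuously in a direction chosen by its MoveType variable.
; Each Tick switches on MoveType and adds full-scale movement input forward, backward, right or left, relative to the actor's current facing.
; The graph never sets MoveType or changes rotation, and the construction script is empty.
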(event EventTick
  (params (DeltaSeconds :type Float%20%28single-precision%29))
  (switch int (Variables|Default|GetMove_type)
    (:1
      (Pawn|Input|AddMovementInput (Transformation|GetActorForwardVector) 1.0 false))
    (:2
      (Pawn|Input|AddMovementInput (Math|Vector|NegateVector (Transformation|GetActorForwardVector)) 1.0 false))
    (:3
      (Pawn|Input|AddMovementInput (Transformation|GetActorRightVector) 1.0 false))
    (:4
      (Pawn|Input|AddMovementInput (Math|Vector|NegateVector (Transformation|GetActorRightVector)) 1.0 false))))

(fn ConstructionScript)