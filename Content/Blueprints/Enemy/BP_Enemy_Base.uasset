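; Base enemy Blueprint that hunts and attacks BP_BaseTeamate actors.
; From BeginPlay, ChasePlayer waits briefly, finds the nearest teammate and uses AIMoveTo to approach it.
; On arrival with a valid target it calls AttackSimple on BasicAttacks, then loops back to pick a target again.
; A failed move or invalid target prints a Polish "cannot find opponent" message and ends the loop.
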(event Custom|ChasePlayer
  (Utilities|FlowControl|Delay 2.0 :!label _label)
  (bind _outactors (Actor|GetAllActorsOfClass "/Game/Blueprints/Teamates/BP_BaseTeamate.BP_BaseTeamate_C"))
  (Variables|Default|SetTarget (.ReturnValue (Actor|FindNearestActor (Transformation|GetActorLocation) _outactors)))
  (AI|AIMoveTo self "0, 0, 0" (.ReturnValue (Actor|FindNearestActor (Transformation|GetActorLocation) _outactors)) (Variables|Default|GetAcceptance%20Radius) false
    (:OnSuccess
      (bind _target (Variables|Default|GetTarget)
        (:then
          (Default|AttackSimple (Variables|Default|GetBasicAttacks) _target 8 0.1 0.1 4.8e+03 1e+01)
          (goto _label))
        (:else
          _)))
    (:OnFail
      _))
  (Development|PrintString "nie można znalezc  przeciwnika"))

(event EventBeginPlay
  (CallFunction|ChasePlayer))

(fn ConstructionScript)