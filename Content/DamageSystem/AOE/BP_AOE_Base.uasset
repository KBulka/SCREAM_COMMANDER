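; BP_AOE_Base is the base area-of-effect actor in the damage system, detecting pawns within a configurable radius around itself.
; Trigger runs the effect, either when called or automatically after a short delay on BeginPlay if enabled.
; It draws a debug sphere, runs a sphere overlap and fires the OnAEOverlapActor dispatcher for each pawn found, applying no damage itself.
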(event Custom|SpawnAOEShpere
  (bind _returnvalue (Transformation|GetActorLocation))
  (bind _sphere_radius (Variables|Default|GetSphere%20Radius))
  (Rendering|Debug|DrawDebugSphere _returnvalue _sphere_radius 12 "(R=0.177083,G=0.000000,B=0.057045,A=1.000000)" 5.0 5.0)
  (bind _outactors (Collision|SphereOverlapActors _returnvalue _sphere_radius (Utilities|Array|MakeArray "ObjectTypeQuery3") 0))
  (for _array_element _outactors
    (Default|CallOnAEOverlapActor _array_element)))

(event Custom|Trigger
  (CallFunction|SpawnAOEShpere))

(event EventBeginPlay
  (if (Variables|Default|GetTriggerOnBeginPlay)
    (Utilities|FlowControl|Delay 0.2)
    (CallFunction|Trigger)))

(fn ConstructionScript)