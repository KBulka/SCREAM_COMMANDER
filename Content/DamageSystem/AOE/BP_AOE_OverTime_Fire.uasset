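; Fire variant of an over-time area-of-effect actor in the damage system.
; Its Trigger event runs the parent logic, then spawns the P_ky_laser01 particle emitter attached to the root component.
; All other behavior, including any damage handling, is left to the parent class, as the remaining events are disabled stubs and construction only calls the parent.
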(event EventBeginPlay
  (|CallParentFunction) ; Ten węzeł jest wyłączony i nie będzie wywoływany.\nPrzeciągnij gniazda, aby utworzyć funkcjonalność.
)

(event Collision|EventActorBeginOverlap
  (params (OtherActor :type Actor%20Object%20Reference))
  (|CallParentFunction OtherActor) ; Ten węzeł jest wyłączony i nie będzie wywoływany.\nPrzeciągnij gniazda, aby utworzyć funkcjonalność.
)

(event EventTick
  (params (DeltaSeconds :type Float%20%28single-precision%29))
  (|CallParentFunction DeltaSeconds) ; Ten węzeł jest wyłączony i nie będzie wywoływany.\nPrzeciągnij gniazda, aby utworzyć funkcjonalność.
)

(event EventTrigger
  (|CallParentFunction)
  (Effects|SpawnEmitterAttached "/Game/FXVarietyPack/Particles/P_ky_laser01.P_ky_laser01" (Variables|Default|GetDefaultSceneRoot) "None"))

(fn ConstructionScript
  (|CallParentFunction))