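; BP_AOE_Attack_Lighting is a delayed area-of-effect attack, apparently a lightning strike, that marks the ground before it hits.
; On BeginPlay it snaps to the floor with a Visibility trace that ignores AttackTarget, using an end point made by scaling the location's Z negatively.
; It shows a decal there, waits DekayBeforStrike, then calls Trigger, which is defined outside this graph, and destroys the decal.
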(event Custom|MoveToFloor
  (bind _returnvalue (Transformation|GetActorLocation))
  (bind (_outhit _returnvalue_2) (Collision|LineTraceByChannel _returnvalue (* _returnvalue "1.000000,1.000000,-10000.000000") "TraceTypeQuery1" false (Utilities|Array|MakeArray (Variables|Default|GetAttack%20Target)) "None"))
  (if _returnvalue_2
    (Transformation|SetActorLocation (.Location (Collision|BreakHitResult _outhit)) false false)))

(event EventBeginPlay
  (|CallParentFunction)
  (CallFunction|MovetoFloor)
  (bind _returnvalue (Rendering|Decal|SpawnDecalatLocation "/Game/StarterContent/Materials/M_Brick_Clay_New.M_Brick_Clay_New" "200.000000,200.000000,250.000000" (Transformation|GetActorLocation) "-90.000000,0.000000,0.000000" 0.0))
  (Utilities|FlowControl|Delay (Variables|Default|GetDekayBeforStrike))
  (CallFunction|Trigger)
  (Components|DestroyComponent _returnvalue))

(event Collision|EventActorBeginOverlap
  (params (OtherActor :type Actor%20Object%20Reference)))

(event EventTick
  (params (DeltaSeconds :type Float%20%28single-precision%29)))

(fn ConstructionScript
  (|CallParentFunction))