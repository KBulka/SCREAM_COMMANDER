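; Actor component that manages health, damage and death for its owner.
; TakeDamage subtracts the damage info's amount, then either sets IsDead and fires OnDeath, or fires DamageResponse with the hit's response type.
; Heal restores health clamped to MaxHealth while alive and prints the result.
; A CanBeDamaged macro gates on death and overridable invincibility, but TakeDamage checks only IsDead.
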(event EventBeginPlay)

(event EventTick
  (params (DeltaSeconds :type Float%20%28single-precision%29)))

(fn Heal
  (params (Amount :type Integer))
  (if (not (Variables|Default|GetIsDead))
    (bind _output_get (Variables|Default|SetHealth (Math|Integer|Clamp(Integer) (+ Amount (Variables|Default|GetHealth)) 0 (Variables|Default|GetMaxHealth))))
    (Development|PrintString (Utilities|String|ToString(Integer) _output_get))
    (return _output_get)))

(fn TakeDamage
  (params (DamageInfo :type S%20Damage%20Info%20Structure))
  (bind (_amount _damagetype _damageresponse) (Utilities|Struct|BreakS_DamageInfo DamageInfo))
  (if (not (Variables|Default|GetIsDead))
    (bind _output_get (Variables|Default|SetHealth (- (Variables|Default|GetHealth) _amount)))
    (if (<= _output_get 0)
      (Variables|Default|SetIsDead true)
      (Default|CallOnDeath)
      (else
        (Default|CallDamageResponse _damageresponse)))
    (return true)))