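; BP_Laser_Base is a base laser actor that draws a Niagara beam between a start actor and an attack target.
; While both references are valid, Tick sets the Beam Start and Beam End parameters to their locations, so the beam follows both actors.
; Tick also runs into a fixed Delay, so the laser destroys itself six seconds after the first valid update.
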(event EventTick
  (params (DeltaSeconds :type Float%20%28single-precision%29))
  (bind _niagara (Variables|Default|GetNiagara))
  ;[1 1 1] Laser Niagra
  (Variables|Default|GetAttackTarget
    (:then
      (Variables|Default|GetStartLocation
        (:then
          (Niagara|SetNiagaraVariable(Vector3) _niagara "Beam End" (Transformation|GetActorLocation (Variables|Default|GetAttackTarget)))
          (Niagara|SetNiagaraVariable(Vector3) _niagara "Beam Start" (Transformation|GetActorLocation (Variables|Default|GetStartLocation)))
          (Utilities|FlowControl|Delay 6.0)
          (Actor|DestroyActor))
        (:else)))
    (:else)))

(fn ConstructionScript)