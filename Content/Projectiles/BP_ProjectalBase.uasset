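; BP_ProjectalBase is a base projectile that damages the actor its Box hits, then spawns an impact effect and explosion sound and destroys itself.
; The construction script feeds Speed and Gravity into ProjectileMovement and enables homing on a valid Target when IsHoming is set.
; On BeginPlay it ignores its owner and aims its velocity at any valid Target, with random spread on world X only.
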(event OnComponentHit(Box)
  (params (HitComponent :type Primitive%20Component%20Object%20Reference) (OtherActor :type Actor%20Object%20Reference) (OtherComp :type Primitive%20Component%20Object%20Reference) (NormalImpulse :type Vector :default "0, 0, 0") (Hit :type Hit%20Result%20Structure%20%28by%20ref%29))
  (bind _location (Collision|BreakHitResult Hit))
  ;[1 1 1] When Enemy is hit
  (CallFunction|DamageEnemy OtherActor)
  (Effects|SpawnEmitteratLocation (Variables|Default|GetimpactEffect) _location)
  (Audio|PlaySoundatLocation "/Game/StarterContent/Audio/Explosion02.Explosion02" _location "0, 0, 0" 0.2 1.0 0.0 0 0 0 0)
  (Actor|DestroyActor))

(event Custom|Rotate%20to%20target
  (bind _target (Variables|Default|GetTarget))
  (bind _returnvalue (Transformation|GetActorLocation _target))
  (bind (_x _y _z) (Math|Vector|BreakVector _returnvalue))
  (Variables|/Script/Engine.MovementComponent|SetVelocity (Variables|Default|GetProjectileMovement) (* (Math|Vector|GetUnitDirection(Vector) (Transformation|GetActorLocation) (Math|Vector|MakeVector (+ _x (Math|Random|RandomFloatinRange -7e+02 7e+02)) _y _z)) (Variables|ProjectileSettings|GetSpeed))))

(event Custom|DamageEnemy
  (params (Other%20Actor :type Actor%20Object%20Reference) (Hit :type Hit%20Result%20Structure))
  ;[1 1 1] Apply damage
  (Class|BPDamageable|TakeDamage(Message) Other%20Actor (Utilities|Struct|MakeS_DamageInfo (Math|Float|Truncate (Variables|ProjectileSettings|GetDamageAmount)) "NewEnumerator1")))

(event EventBeginPlay
  (Collision|IgnoreActorwhenMoving (Variables|Default|GetBox) (Components|GetOwner) true)
  (Variables|Default|GetTarget
    (:then
      (CallFunction|RotatetoTarget))
    (:else)))

(fn ConstructionScript
  (bind _projectilemovement (Variables|Default|GetProjectileMovement))
  (Variables|/Script/Engine.ProjectileMovementComponent|SetInitialSpeed _projectilemovement (Variables|ProjectileSettings|GetSpeed))
  (Variables|/Script/Engine.ProjectileMovementComponent|SetMaxSpeed _projectilemovement (Variables|ProjectileSettings|GetSpeed))
  (Variables|/Script/Engine.ProjectileMovementComponent|SetProjectileGravityScale _projectilemovement (Variables|ProjectileSettings|GetGravity))
  (Variables|Default|GetTarget
    (:then
      (if (Variables|Default|GetisHoming)
        (Variables|/Script/Engine.ProjectileMovementComponent|SetbIsHomingProjectile _projectilemovement true)
        (Variables|/Script/Engine.ProjectileMovementComponent|SetHomingTargetComponent _projectilemovement (Variables|/Script/Engine.Actor|GetRootComponent (Variables|Default|GetTarget)))))
    (:else)))